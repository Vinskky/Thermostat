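; EnemyShoot_BP is an enemy actor whose model spins every Tick and roams between six Arrow component positions; it contains no shooting logic.
; FindNextPosition picks a random arrow's world location as the target, calls Moving, then repeats after a short random delay.
; Moving re-arms its own timer and resets Alpha on each pass, so each step lerps a small fixed fraction from the current location, easing toward the target.
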(event Custom|Moving
  (bind _model (Variables|Default|GetModel))
  (Variables|Default|SetAlpha 0.0)
  (Utilities|Time|SetTimerbyEvent (delegate Custom|Moving) 0.02)
  (Variables|Default|SetAlpha (+ (Variables|Default|GetAlpha) 0.04))
  (Transformation|SetWorldLocation _model (Math|Vector|Lerp(Vector) (Transformation|GetWorldLocation _model) (Variables|Default|GetLocationToMove) (Variables|Default|GetAlpha)) false false))

(event Custom|FindNextPosition
  (bind _arrow5 (Variables|Default|GetArrow5))
  (bind _arrow3 (Variables|Default|GetArrow3))
  (bind _arrow4 (Variables|Default|GetArrow4))
  (bind _arrow2 (Variables|Default|GetArrow2))
  (bind _arrow1 (Variables|Default|GetArrow1))
  (bind _arrow (Variables|Default|GetArrow))
  (bind _array (Utilities|Array|MakeArray _arrow5 _arrow4 _arrow3 _arrow2 _arrow1 _arrow))
  (Variables|Default|SetLocationToMove (Transformation|GetWorldLocation (Utilities|Array|Get(acopy) _array (Math|Random|RandomIntegerinRange 0 (Utilities|Array|LastIndex _array)))))
  (CallFunction|Moving)
  (Utilities|FlowControl|Delay (Math|Random|RandomFloatinRange 1.5 2.5))
  (CallFunction|FindNextPosition))

(event EventTick
  (params (DeltaSeconds :type Float%20%28single-precision%29))
  (Transformation|AddLocalRotation (Variables|Default|GetModel) (Math|Rotator|MakeRotator 0.0 0.0 (Variables|Default|GetDelta%20Rotation%20Z%20%28Yaw%29)) false false))

(event EventBeginPlay
  (CallFunction|FindNextPosition))

(fn ConstructionScript)